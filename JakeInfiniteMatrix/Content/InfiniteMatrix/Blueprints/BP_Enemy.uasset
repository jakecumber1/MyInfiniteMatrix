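; BP_Enemy is a short-lived enemy actor that damages the player on contact and awards score through its projectile-damage function.
; Capsule hit and begin-overlap events share a cast to BP_Player, then HitPlayer calls TakeDamage on the player and destroys the enemy.
; DamageFromProj, not called within this Blueprint, increases the player's score and destroys the enemy.
; The construction script sets a brief lifespan so untouched enemies expire automatically.
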(event OnComponentHit(Capsule)
  (params (HitComponent :type Primitive%20Component%20Object%20Reference) (OtherActor :type Actor%20Object%20Reference) (OtherComp :type Primitive%20Component%20Object%20Reference) (NormalImpulse :type Vector :default "0, 0, 0") (Hit :type Hit%20Result%20Structure%20%28by%20ref%29))
  (Utilities|Casting|CastToBP_Player OtherActor)
  (CallFunction|HitPlayer))

(event OnComponentBeginOverlap(Capsule)
  (params (OverlappedComponent :type Primitive%20Component%20Object%20Reference) (OtherActor :type Actor%20Object%20Reference) (OtherComp :type Primitive%20Component%20Object%20Reference) (OtherBodyIndex :type Integer) (bFromSweep :type Boolean) (SweepResult :type Hit%20Result%20Structure%20%28by%20ref%29))
  (Utilities|Casting|CastToBP_Player (stale OnComponentHit(Capsule) OtherActor))
  (CallFunction|HitPlayer))

(event EventBeginPlay)

(event Collision|EventActorBeginOverlap
  (params (OtherActor :type Actor%20Object%20Reference)))

(event EventTick
  (params (DeltaSeconds :type Float%20%28single-precision%29)))

(fn ConstructionScript
  (Actor|SetLifeSpan 3.0))

(fn DamagefromProj
  (bind _asbp_player (Utilities|Casting|CastToBP_Player (Game|Player|GetPlayerPawn 0)))
  (Default|IncreaseScore _asbp_player)
  (Actor|DestroyActor))

(fn HitPlayer
  (bind _asbp_player (Utilities|Casting|CastToBP_Player (Game|Player|GetPlayerPawn 0)))
  (Default|TakeDamage _asbp_player)
  (Actor|DestroyActor))