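; BP_Tunnel is a tunnel segment with a rotating holed wall that the player must pass.
; RandomizeWall picks one of four hole meshes, colored by the player's Health, and applies a random roll.
; Reaching the trigger zone has TunnelSpawner spawn another tunnel, increases score and destroys this segment.
; Wall overlaps call StopScore on the player or destroy projectiles.
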(event OnComponentBeginOverlap(TriggerZone)
  (params (OverlappedComponent :type Primitive%20Component%20Object%20Reference) (OtherActor :type Actor%20Object%20Reference) (OtherComp :type Primitive%20Component%20Object%20Reference) (OtherBodyIndex :type Integer) (bFromSweep :type Boolean) (SweepResult :type Hit%20Result%20Structure%20%28by%20ref%29))
  (bind _asbp_player (Utilities|Casting|CastToBP_Player OtherActor))
  (Default|SpawnTunnelatPoint (Variables|Default|GetTunnelSpawner))
  (Default|IncreaseScore _asbp_player)
  (Actor|DestroyActor))

(event OnComponentBeginOverlap(WallMesh)
  (params (OverlappedComponent :type Primitive%20Component%20Object%20Reference) (OtherActor :type Actor%20Object%20Reference) (OtherComp :type Primitive%20Component%20Object%20Reference) (OtherBodyIndex :type Integer) (bFromSweep :type Boolean) (SweepResult :type Hit%20Result%20Structure%20%28by%20ref%29))
  (bind _asbp_player (Utilities|Casting|CastToBP_Player OtherActor)
    (:then
      (Default|StopScore _asbp_player))
    (:CastFailed
      (bind _asbp_projectile (Utilities|Casting|CastToBP_Projectile OtherActor))
      (Actor|DestroyActor _asbp_projectile))))

(event EventBeginPlay)

(event EventTick
  (params (DeltaSeconds :type Float%20%28single-precision%29))
  (Transformation|AddLocalRotation (Variables|Default|GetWallMesh) (Math|Rotator|MakeRotator (* DeltaSeconds (Variables|Default|GetRotateSpeed)) 0.0 0.0) false false))

(fn ConstructionScript)

(fn RandomizeWall
  (bind _wallmesh (Variables|Default|GetWallMesh))
  (bind _asbp_player (Utilities|Casting|CastToBP_Player (Game|Player|GetPlayerPawn 0)))
  (if (== (Variables|/Game/InfiniteMatrix/Blueprints/BP_Player.BP_Player_C|GetHealth _asbp_player) 3.0)
    (Components|StaticMesh|SetStaticMesh _wallmesh (Utilities|Select :Index (Math|Random|RandomIntegerinRange 0 3) :Option%200 "/Game/InfiniteMatrix/Meshes/SM_Hole_01.SM_Hole_01" :Option%201 "/Game/InfiniteMatrix/Meshes/SM_Hole_02.SM_Hole_02" :Option%202 "/Game/InfiniteMatrix/Meshes/SM_Hole_03.SM_Hole_03" :Option%203 "/Game/InfiniteMatrix/Meshes/SM_Hole_04.SM_Hole_04"))
    (elif (== (Variables|/Game/InfiniteMatrix/Blueprints/BP_Player.BP_Player_C|GetHealth _asbp_player) 2.0)
      (Components|StaticMesh|SetStaticMesh (Variables|Default|GetWallMesh) (Utilities|Select :Index (Math|Random|RandomIntegerinRange 0 3) :Option%200 "/Game/InfiniteMatrix/Meshes/SM_Hole_01_Purp.SM_Hole_01_Purp" :Option%201 "/Game/InfiniteMatrix/Meshes/SM_Hole_02_Purp.SM_Hole_02_Purp" :Option%202 "/Game/InfiniteMatrix/Meshes/SM_Hole_03_Purp.SM_Hole_03_Purp" :Option%203 "/Game/InfiniteMatrix/Meshes/SM_Hole_04_Purp.SM_Hole_04_Purp"))
      (else
        (Components|StaticMesh|SetStaticMesh (Variables|Default|GetWallMesh) (Utilities|Select :Index (Math|Random|RandomIntegerinRange 0 3) :Option%200 "/Game/InfiniteMatrix/Meshes/SM_Hole_01_Red.SM_Hole_01_Red" :Option%201 "/Game/InfiniteMatrix/Meshes/SM_Hole_02_Red.SM_Hole_02_Red" :Option%202 "/Game/InfiniteMatrix/Meshes/SM_Hole_03_Red.SM_Hole_03_Red" :Option%203 "/Game/InfiniteMatrix/Meshes/SM_Hole_04_Red.SM_Hole_04_Red")))))
  (Transformation|AddLocalRotation _wallmesh (Math|Rotator|MakeRotator (Math|Random|RandomFloatinRange 0.0 3.6e+02) 0.0 0.0) false false))