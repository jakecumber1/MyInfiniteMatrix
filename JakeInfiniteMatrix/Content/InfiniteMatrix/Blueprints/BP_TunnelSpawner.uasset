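; BP_TunnelSpawner builds a chain of BP_Tunnel segments, populated with enemies and health packs.
; On BeginPlay it clears existing tunnels and, in loops nested under that, enemies and health packs, then spawns the initial segments from the player's location.
; SpawnTunnelAtPoint extends the chain at the newest tunnel's SpawnPoint.
; Each tunnel receives a spawner reference, randomizes its wall and randomly gets enemies and a health pack at offset positions.
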(event EventBeginPlay
  (CallFunction|SpawnInitialTunnels))

(event Collision|EventActorBeginOverlap
  (params (OtherActor :type Actor%20Object%20Reference)))

(event EventTick
  (params (DeltaSeconds :type Float%20%28single-precision%29)))

(fn ConstructionScript)

(fn SpawnTunnel
  (params (SpawnLocation :type Vector))
  (bind _returnvalue (Math|Random|RandomInteger 3))
  (bind _returnvalue_2 (Game|SpawnActorfromClass "/Game/InfiniteMatrix/Blueprints/BP_Tunnel.BP_Tunnel_C" (Math|Transform|MakeTransform SpawnLocation "0, 0, 0" "1.000000,1.000000,1.000000") "Undefined" 0 0))
  (bind _output_get (Variables|Default|SetNewestTunnel _returnvalue_2))
  (Variables|/Game/InfiniteMatrix/Blueprints/BP_Tunnel.BP_Tunnel_C|SetTunnelSpawner _output_get self)
  (Default|RandomizeWall _output_get)
  (if (== _returnvalue 0)
    _
    (else
      (for _index (range 0 _returnvalue)
        (CallFunction|SpawnEnemy SpawnLocation))))
  (if (== (Math|Random|RandomInteger 4) 3)
    (CallFunction|SpawnHealthPack (+ SpawnLocation (Math|Vector|MakeVector (Math|Random|RandomFloatinRange -375.0 -5e+02) (Math|Random|RandomFloatinRange -2e+02 2e+02) (Math|Random|RandomFloatinRange -4e+02 4e+02))))))

(fn SpawnTunnelatPoint
  (CallFunction|SpawnTunnel (Transformation|GetWorldLocation (Variables|/Game/InfiniteMatrix/Blueprints/BP_Tunnel.BP_Tunnel_C|GetSpawnPoint (Variables|Default|GetNewestTunnel))))
  (if (== (Math|Random|RandomInteger 1) 0)
    _))

(fn SpawnInitialTunnels
  (Utilities|FlowControl|Sequence
    (:then_0
      (bind _outactors (Actor|GetAllActorsOfClass "/Game/InfiniteMatrix/Blueprints/BP_Tunnel.BP_Tunnel_C"))
      (for _array_element _outactors
        (Actor|DestroyActor _array_element)
        (bind _outactors_2 (Actor|GetAllActorsOfClass "/Game/InfiniteMatrix/Blueprints/BP_Enemy.BP_Enemy_C"))
        (for _array_element_2 _outactors_2
          (Actor|DestroyActor _array_element_2)
          (bind _outactors_3 (Actor|GetAllActorsOfClass "/Game/InfiniteMatrix/Blueprints/BP_HealthPack.BP_HealthPack_C"))
          (for _array_element_3 _outactors_3
            (Actor|DestroyActor _array_element_3)))))
    (:then_1
      (for _index (range 0 2)
        (Utilities|IsValid (Variables|Default|GetNewestTunnel)
          (:Is%20Valid
            (CallFunction|SpawnTunnelatPoint))
          (:Is%20Not%20Valid
            (CallFunction|SpawnTunnel (Transformation|GetActorLocation (Game|Player|GetPlayerPawn 0)))))))))

(fn SpawnHealthPack
  (params (SpawnLocation :type Vector))
  (Game|SpawnActorfromClass "/Game/InfiniteMatrix/Blueprints/BP_HealthPack.BP_HealthPack_C" (Math|Transform|MakeTransform SpawnLocation "0, 0, 0" "1.000000,1.000000,1.000000") "Undefined" 0 0))

(fn SpawnEnemy
  (params (SpawnLocation :type Vector))
  (Game|SpawnActorfromClass "/Game/InfiniteMatrix/Blueprints/BP_Enemy.BP_Enemy_C" (Math|Transform|MakeTransform (+ SpawnLocation (Math|Vector|MakeVector (Math|Random|RandomFloatinRange -5e+02 -1e+03) (Math|Random|RandomFloatinRange -1.5e+02 1.5e+02) (Math|Random|RandomFloatinRange -3e+02 3e+02))) "0, 0, 0" "1.000000,1.000000,1.000000") "Undefined" 0 0))